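; BP_EnemySpawnPoint is a spawn point actor meant to spawn a BP_EnemyAI at its own transform after a timed delay.
; Tick accumulates delta time and spawns only when the total exactly equals the threshold, a float comparison that rarely matches, and the timer never resets.
; It reads EnemyLimit from the GameStatic game instance, but the branch before spawning is always true, so the limit is not enforced.
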(event `self.ReceiveBeginPlay`)

(event `self.ReceiveTick`
  (params (DeltaSeconds :type "Float (single-precision)"))
  (set `self.TimeToSpawn` (+ (`self.TimeToSpawn`) DeltaSeconds))
  (if (== (`self.TimeToSpawn`) 20.0)
    (bind _asgame_static (cast `/Game/Blueprint/GameStatic` (`GameplayStatics.GetGameInstance`)))
    (set `self.num` (`/Game/Blueprint/GameStatic.Enemy_limit` _asgame_static))
    (if true
      (`|SpawnActorFromClass` "/Game/Blueprint/BP_EnemyAI.BP_EnemyAI_C" (`self.GetTransform`) "Undefined" "MultiplyWithRoot" null null))))

(fn `UserConstructionScript`)